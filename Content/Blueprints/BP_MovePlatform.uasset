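; BP_MovePlatform is a gimmick-driven platform that moves vertically when activated and returns when deactivated.
; BeginPlay caches the starting world Z and sets the timeline to half speed.
; Gimmick activation plays the timeline and deactivation reverses it, with its Alpha scaled by MoveDistance as the Z offset.
; The result is applied through SetActorRelativeLocation using world coordinates, so it assumes relative and world space match.
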(event `self.ReceiveBeginPlay`
  (bind (_returnvalue_x _returnvalue_y _returnvalue_z) (`KismetMathLibrary.BreakVector` (`self.K2_GetActorLocation`)))
  (set `self.LocationZ` _returnvalue_z)
  (`TimelineComponent.SetPlayRate` (`self.Timeline`) 0.5))

(event `self.OnGimmickActivated`
  (bind (_returnvalue_x _returnvalue_y) (`KismetMathLibrary.BreakVector` (`self.K2_GetActorLocation`)))
  (bind (_direction _alpha) (`Timeline|Timeline` :!label _label)
    (:`Update`
      (`self.K2_SetActorRelativeLocation` (`KismetMathLibrary.MakeVector` _returnvalue_x _returnvalue_y (+ (`self.LocationZ`) (* _alpha (`self.MoveDistance`))))))))

(event `self.OnGimmickDeactivated`
  (goto _label :!via `Reverse`))

(fn `UserConstructionScript`)